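; BP_EnemySpawner is an actor that spawns a limited number of NPC_Test enemies around its location.
; A looping timer set on BeginPlay fires every few seconds, but only spawns while StartSpawning is true.
; Each spawn uses a random navmesh-reachable point within a wide radius and decrements NumberOfEnemies.
; The timer is cleared once that count is used up.
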(event `self.ReceiveBeginPlay`
  (bind _returnvalue (`KismetSystemLibrary.K2_SetTimerDelegate` (delegate `Spawn Enemy`) 5.0 true)))

(event `Spawn Enemy`
  (if (`self.StartSpawning`)
    (`|SpawnActorFromClass` "/Game/Blueprints/NPC_Test.NPC_Test_C" (`KismetMathLibrary.MakeTransform` (`NavigationSystemV1.K2_GetRandomReachablePointInRadius` (`self.K2_GetActorLocation`) 7000.0 null null)) "Undefined" "MultiplyWithRoot" null 10.0 true false null)
    (bind _output_get (set `self.NumberOfEnemies` (- (`self.NumberOfEnemies`) 1)))
    (if (<= _output_get 0)
      (`KismetSystemLibrary.K2_ClearAndInvalidateTimerHandle` (stale `self.ReceiveBeginPlay` _returnvalue)))))

(fn `UserConstructionScript`)