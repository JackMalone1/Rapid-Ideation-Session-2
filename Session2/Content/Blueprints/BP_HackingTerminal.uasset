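; BP_HackingTerminal is an interactable hacking terminal that opens a dialogue conversation when used.
; SetInteractableState shows or hides its Name component to match whether interaction is available.
; Interact stores the instigator and opens the conversation through the ACDialogueTerminal component.
; When the conversation closes, it notifies that stored instigator through ConversationClosedMessage.
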(event `/Game/Blueprints/BP_Interactable.SetInteractableState`
  (params (`bCanShowInteract?` :type Boolean))
  (if `bCanShowInteract?`
    (`SceneComponent.SetVisibility` (`self.Name`) true false)
    (else
      (`SceneComponent.SetVisibility` (`self.Name`) false false))))

(event `/Game/Blueprints/BP_Interactable.Interact`
  (params (Instigator :type "Actor Object Reference"))
  (set `self.Interact Instigator` Instigator)
  (`/Game/Blueprints/AC_Dialogue_base.OpenConversation` (`self.AC_Dialogue_Terminal`)))

(event `/Game/Blueprints/BP_Interactable.ConversationClosed`
  (message `/Game/Blueprints/BP_Interactable.ConversationClosed` (`self.Interact Instigator`)))

(fn `UserConstructionScript`)