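; NPC_Test is a test NPC character that can be talked to and killed.
; Interact stores the instigator and opens a conversation through the ACDialogueTest component while the NPC is interactable.
; AnyDamage subtracts from Health, and at zero or below the mesh ragdolls through physics simulation, movement stops, interaction is disabled and the NPC is marked dead.
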(event `/Game/Blueprints/BP_Interactable.Interact`
  (params (Instigator :type "Actor Object Reference"))
  (if (`self.Interactable`)
    (set `self.InteractInstigator` Instigator)
    (`/Game/Blueprints/AC_Dialogue_base.OpenConversation` (`self.AC_Dialogue_Test`))))

(event `self.ReceiveAnyDamage`
  (params (Damage :type "Float (single-precision)") (DamageType :type "DamageType Object Reference") (InstigatedBy :type "Controller Object Reference") (DamageCauser :type "Actor Object Reference"))
  (set `self.Health` (- (`self.Health`) Damage))
  (if (<= (`self.Health`) 0.0)
    (`PrimitiveComponent.SetSimulatePhysics` (`self.Mesh`) true)
    (`CharacterMovementComponent.SetMovementMode` (`self.CharacterMovement`) "MOVE_None" 0)
    (set `self.Interactable` false)
    (set `self.IsDead?` true)))

(fn `UserConstructionScript`
  (`parent.UserConstructionScript`))