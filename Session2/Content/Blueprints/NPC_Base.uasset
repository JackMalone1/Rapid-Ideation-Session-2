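; Base NPC that shows a name label when interactable, relays conversation closure to its instigator, and can act as a rifle-armed enemy.
; With SearchAround on, it roams random reachable points until PawnSensing spots the player character, then chases and fires a damaging, debug-drawn line trace from the muzzle along the mesh's right vector.
; A quarter-second loop re-runs Search and clears the seen-target flag, so roaming resumes without fresh sightings.
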(event `/Game/Blueprints/BP_Interactable.SetInteractableState`
  (params (`bCanShowInteract?` :type Boolean))
  (if `bCanShowInteract?`
    (`SceneComponent.SetVisibility` (`self.CharacterName`) true false)
    (else
      (`SceneComponent.SetVisibility` (`self.CharacterName`) false false))))

(event `/Game/Blueprints/BP_Interactable.ConversationClosed`
  (message `/Game/Blueprints/BP_Interactable.ConversationClosed` (`self.InteractInstigator`)))

(event `Search`
  (if (and (not (`self.HasSeenTarget?`)) (`self.SearchAround`))
    (`|AIMoveTo` self (`NavigationSystemV1.K2_GetRandomReachablePointInRadius` (`self.K2_GetActorLocation`) 2000.0 null null) null 600.0
      (:`OnSuccess`
        (`KismetSystemLibrary.Delay` 1.0)
        (`self.Search`)))))

(event `self.ReceiveBeginPlay`
  (`self.Search`)
  (`KismetSystemLibrary.Delay` 0.25 :!label _label)
  (`self.Search`)
  (set `self.HasSeenTarget?` false)
  (goto _label))

(event `self.PawnSensing.OnSeePawn`
  (params (Pawn :type "Pawn Object Reference"))
  (if (`self.SearchAround`)
    (bind _asbp_third_person_character (cast `/Game/ThirdPerson/Blueprints/BP_ThirdPersonCharacter` Pawn))
    (`self.Chase` _asbp_third_person_character)
    (set `self.HasSeenTarget?` true)))

(event `Chase`
  (params (TargetActor :type "Actor Object Reference"))
  (`|AIMoveTo` self (0.0 0.0 0.0) TargetActor 300.0
    (:`OnSuccess`
      (`self.Fire` TargetActor))))

(event `Fire`
  (params (TargetActor :type "Actor Object Reference"))
  (bind _returnvalue_location (`KismetMathLibrary.BreakTransform` (`SceneComponent.GetSocketTransform` (`self.Rifle`) "b_gun_muzzleflash" "RTS_World")))
  (if (not (`self.IsDead?`))
    (`Controller.SetControlRotation` (`self.GetController`) (`KismetMathLibrary.FindLookAtRotation` (`self.K2_GetActorLocation`) (`self.K2_GetActorLocation` TargetActor)))
    (bind (_outhit _returnvalue) (`KismetSystemLibrary.LineTraceSingle` :`Start` _returnvalue_location :`End` (+ _returnvalue_location (* (`KismetMathLibrary.GetRightVector` (`SceneComponent.K2_GetComponentRotation` (`self.Mesh`))) 3000.0)) :`TraceChannel` "TraceTypeQuery1" :`DrawDebugType` "ForDuration"))
    (if _returnvalue
      (`GameplayStatics.ApplyDamage` (`.HitActor` (`GameplayStatics.BreakHitResult` _outhit)) 5.0))))

(fn `UserConstructionScript`
  (`TextRenderComponent.K2_SetText` (`self.CharacterName`) (`self.TextCharacterName`)))