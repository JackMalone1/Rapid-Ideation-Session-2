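; Test dialogue component that defines a small sample conversation with a two-option branch.
; It overrides Dialogue, calls the parent, then switches on DialogueTreeIndex, with index 0 and default sharing one tree.
; Chained AddDialogue calls advance only on their Pass Through state, with the first option index choosing the follow-up line.
; Each follow-up shows options again, then clears dialogue progress and closes the conversation.
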(fn `Dialogue`
  (`parent.Dialogue`)
  (switch `int` (`self.DialogueTreeIndex`)
    (:`Default`
      _)
    (:`0`
      _))
  (bind (_state _option_index) (`self.AddDialogue` "Test" "This is a test sentence" (`|MakeArray` "First Response" "Second Response" :!type "Text")))
  (switch `/Game/Blueprints/Enum_DialogueState` _state
    (:`NewEnumerator0`
      (switch `int` _option_index
        (:`0`
          (bind (_state_2 _option_index_2) (`self.AddDialogue` "Test" "First option was selected" (`|MakeArray` "First Response" "Second Response" :!type "Text")))
          (switch `/Game/Blueprints/Enum_DialogueState` _state_2
            (:`NewEnumerator0`
              (switch `int` _option_index_2
                (:`Default`
                  (`self.ClearDialogueProgress`)
                  (`self.CloseConversation`))))))
        (:`1`
          (bind _state_3 (`self.AddDialogue` "Test" "Second Option was selected" (`|MakeArray` "First Response" "Second Response" :!type "Text")))
          (switch `/Game/Blueprints/Enum_DialogueState` _state_3
            (:`NewEnumerator0`
              (`self.ClearDialogueProgress`)
              (`self.CloseConversation`))))))))